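; BaseWeapon is a weapon base Blueprint that provides single-trace hitscan shooting.
; StartShooting line-traces on the Camera channel from the ProjectileDirection component along its forward vector, out to ShootingRange.
; A hit applies Damage of DamageType to the hit actor, always crediting player controller 0 as instigator and the weapon as causer.
; StopShooting is an empty event, and construction adds no logic.
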(event Custom|StartShooting
  (bind _projectiledirection (Variables|Default|GetProjectileDirection))
  (bind _returnvalue (Transformation|GetWorldLocation _projectiledirection))
  (bind (_outhit _returnvalue_2) (Collision|LineTraceByChannel _returnvalue (+ _returnvalue (* (Math|Vector|GetForwardVector _projectiledirection) (Variables|Default|GetShootingRange))) "TraceTypeQuery2" false 0 "None"))
  (if _returnvalue_2
    (Game|Damage|ApplyDamage (.HitActor (Collision|BreakHitResult _outhit)) (Variables|Default|GetDamage) (Game|GetPlayerController 0) self "/Script/Engine.DamageType")))

(event Custom|StopShooting)

(event EventBeginPlay)

(event Collision|EventActorBeginOverlap
  (params (OtherActor :type Actor%20Object%20Reference)))

(event EventTick
  (params (DeltaSeconds :type Float%20%28single-precision%29)))

(fn ConstructionScript)