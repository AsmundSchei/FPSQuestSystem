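; Quest log Blueprint that stores the player's quests and toggles the quest log screen.
; AddQuestToLog adds quests without duplicates.
; OpenQuestLog either removes the existing widget and restores game-only input, or plays a sound and creates one stretched across the MainPlayerController's HUD canvas.
; While open, the widget takes UI-only input with the cursor shown and mouse locked.
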(event EventBeginPlay)

(event EventTick
  (params (DeltaSeconds :type Float%20%28single-precision%29)))

(fn AddQuesttoLog
  (params (Quest :type Base%20Quest%20Object%20Reference))
  (Utilities|Array|AddUnique (Variables|Default|GetQuest) Quest))

(fn OpenQuestLog
  (bind _returnvalue (Game|GetPlayerController 0))
  (bind _returnvalue_2 (Game|GetPlayerController 0))
  (bind _questlogwidget (Variables|Default|GetQuestLogWidget)
    (:then
      (Widget|RemovefromParent _questlogwidget)
      (Variables|Default|SetQuestLogWidget 0)
      (Input|SetInputModeGameOnly _returnvalue_2)
      (Variables|/Script/Engine.PlayerController|SetbShowMouseCursor _returnvalue_2 false))
    (:else
      (Audio|PlaySound2D "/Engine/VREditor/Sounds/UI/Selection_Changes.Selection_Changes" 1.0 1.0 0.0 0 0)
      (bind _returnvalue_3 (UserInterface|CreateWidget "/Game/Game/Blueprints/QuestSystem/Widgets/QuestLogWidget.QuestLogWidget_C"))
      (Variables|Default|SetQuestLogWidget _returnvalue_3)
      (bind _asmain_player_controller (Utilities|Casting|CastToMainPlayerController _returnvalue_2))
      (bind _returnvalue_4 (Class|CanvasPanel|AddChildtoCanvas (Variables|/Game/Game/Blueprints/MainPlayerController.MainPlayerController_C|GetMainHudCanvasPanel _asmain_player_controller) (Variables|Default|GetQuestLogWidget)))
      (Class|CanvasPanelSlot|SetAnchors _returnvalue_4 (Utilities|Struct|MakeAnchors "(X=0.000000,Y=0.000000)" "(X=1.000000,Y=1.000000)"))
      (Input|SetInputModeUIOnly _returnvalue (Variables|Default|GetQuestLogWidget) "LockAlways")
      (Variables|/Script/Engine.PlayerController|SetbShowMouseCursor _returnvalue true))))