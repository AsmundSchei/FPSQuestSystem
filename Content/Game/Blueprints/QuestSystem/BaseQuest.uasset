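; Base quest actor that tracks an array of location, interaction, collection and kill objectives for the player.
; On BeginPlay it caches the player's Inventory and binds events for each objective type.
; Check functions match targets by reference or class, using inventory amounts or one shared kill counter, then rewrite matching objective structs and refresh the HUD objectives widget.
; AdjustEditorLocation moves the quest to its parent actor's location.
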(event EventBeginPlay
  (bind _asfirst_person_character (Utilities|Casting|CastToFirstPersonCharacter (Game|GetPlayerCharacter 0)))
  (Variables|Default|SetInventory (Variables|/Game/Game/Blueprints/FirstPersonCharacter.FirstPersonCharacter_C|GetInventory _asfirst_person_character))
  (EventDispatchers|BindEventtoReachedLocation (EventDispatchers|CreateEvent :!event CheckObjectiveLocation))
  (EventDispatchers|BindEventtoInteractionCompleted (EventDispatchers|CreateEvent :!event CheckObjectiveInteraction))
  (EventDispatchers|BindEventtoCollectionCompleted (EventDispatchers|CreateEvent :!event CheckObjectiveCollection))
  (EventDispatchers|BindEventtoKillCompleted (EventDispatchers|CreateEvent :!event CheckObjectiveKillCount)))

(event Collision|EventActorBeginOverlap
  (params (OtherActor :type Actor%20Object%20Reference)))

(event EventTick
  (params (DeltaSeconds :type Float%20%28single-precision%29)))

(fn ConstructionScript)

(fn AdjustEditorLocation
  (Transformation|SetActorLocation (Transformation|GetActorLocation (Actor|GetParentActor)) false false))

(fn CheckObjectiveLocation
  (params (LocationTarget :type Location%20Marker%20Object%20Reference))
  (for (_array_element _array_index) (Variables|QuestInfo|GetObjectives)
    (LocalVariables|SetObjectiveNumberLocal _array_index)
    (if (and (not (.Questcomplete (Utilities|Struct|BreakObjectiveInfo _array_element))) (== (.ObjectiveTarget (Utilities|Struct|BreakObjectiveInfo _array_element)) LocationTarget))
      (Utilities|Array|SetArrayElem (Variables|QuestInfo|GetObjectives) (LocalVariables|GetObjectiveNumberLocal) (Utilities|Struct|MakeObjectiveInfo (.description (Utilities|Array|Get(acopy) (Variables|QuestInfo|GetObjectives) (LocalVariables|GetObjectiveNumberLocal))) (.type (Utilities|Array|Get(acopy) (Variables|QuestInfo|GetObjectives) (LocalVariables|GetObjectiveNumberLocal))) (.amount (Utilities|Array|Get(acopy) (Variables|QuestInfo|GetObjectives) (LocalVariables|GetObjectiveNumberLocal))) (.objectivetarget (Utilities|Array|Get(acopy) (Variables|QuestInfo|GetObjectives) (LocalVariables|GetObjectiveNumberLocal))) true))
      (LocalVariables|SetUpdateQuestStatusLocal true)))
  (if (LocalVariables|GetUpdateQuestStatusLocal)
    (bind _asmain_player_controller (Utilities|Casting|CastToMainPlayerController (Game|GetPlayerController 0)))
    (Default|UpdateObjectiveState (Variables|/Game/Game/Blueprints/Widgets/MainGameWidget.MainGameWidget_C|GetObjectivesBoxWidget (Variables|/Game/Game/Blueprints/MainPlayerController.MainPlayerController_C|GetMainGameWidget _asmain_player_controller)))))

(fn CheckObjectiveInteraction
  (params (InteractorTarget :type Actor%20Object%20Reference))
  (for (_array_element _array_index) (Variables|QuestInfo|GetObjectives)
    (LocalVariables|SetObjectiveNumberLocal _array_index)
    (if (and (not (.Questcomplete (Utilities|Struct|BreakObjectiveInfo _array_element))) (== (.ObjectiveTarget (Utilities|Struct|BreakObjectiveInfo _array_element)) InteractorTarget))
      (Utilities|Array|SetArrayElem (Variables|QuestInfo|GetObjectives) (LocalVariables|GetObjectiveNumberLocal) (Utilities|Struct|MakeObjectiveInfo (.description (Utilities|Array|Get(acopy) (Variables|QuestInfo|GetObjectives) (LocalVariables|GetObjectiveNumberLocal))) (.type (Utilities|Array|Get(acopy) (Variables|QuestInfo|GetObjectives) (LocalVariables|GetObjectiveNumberLocal))) (.amount (Utilities|Array|Get(acopy) (Variables|QuestInfo|GetObjectives) (LocalVariables|GetObjectiveNumberLocal))) (.objectivetarget (Utilities|Array|Get(acopy) (Variables|QuestInfo|GetObjectives) (LocalVariables|GetObjectiveNumberLocal))) true))
      (LocalVariables|SetUpdateQuestStatusLocal true)))
  (if (LocalVariables|GetUpdateQuestStatusLocal)
    (bind _asmain_player_controller (Utilities|Casting|CastToMainPlayerController (Game|GetPlayerController 0)))
    (Default|UpdateObjectiveState (Variables|/Game/Game/Blueprints/Widgets/MainGameWidget.MainGameWidget_C|GetObjectivesBoxWidget (Variables|/Game/Game/Blueprints/MainPlayerController.MainPlayerController_C|GetMainGameWidget _asmain_player_controller)))))

(fn CheckObjectiveCollection
  (params (ItemTarget :type Base%20Item%20Object%20Reference))
  (for (_array_element _array_index) (Variables|QuestInfo|GetObjectives)
    (LocalVariables|SetObjectiveNumberLocal _array_index)
    (if (== (Utilities|GetClass (.ObjectiveTarget (Utilities|Struct|BreakObjectiveInfo _array_element))) (Utilities|GetClass ItemTarget))
      (bind _isininventory (Default|Check (Variables|Default|GetInventory) (Utilities|GetClass ItemTarget) (.Amount (Utilities|Struct|BreakObjectiveInfo _array_element))))
      (if _isininventory
        (Utilities|Array|SetArrayElem (Variables|QuestInfo|GetObjectives) (LocalVariables|GetObjectiveNumberLocal) (Utilities|Struct|MakeObjectiveInfo (.description (Utilities|Array|Get(acopy) (Variables|QuestInfo|GetObjectives) (LocalVariables|GetObjectiveNumberLocal))) (.type (Utilities|Array|Get(acopy) (Variables|QuestInfo|GetObjectives) (LocalVariables|GetObjectiveNumberLocal))) (.amount (Utilities|Array|Get(acopy) (Variables|QuestInfo|GetObjectives) (LocalVariables|GetObjectiveNumberLocal))) (.objectivetarget (Utilities|Array|Get(acopy) (Variables|QuestInfo|GetObjectives) (LocalVariables|GetObjectiveNumberLocal))) true))
        (LocalVariables|SetUpdateQuestStatusLocal true))))
  (if (LocalVariables|GetUpdateQuestStatusLocal)
    (bind _asmain_player_controller (Utilities|Casting|CastToMainPlayerController (Game|GetPlayerController 0)))
    (Default|UpdateObjectiveState (Variables|/Game/Game/Blueprints/Widgets/MainGameWidget.MainGameWidget_C|GetObjectivesBoxWidget (Variables|/Game/Game/Blueprints/MainPlayerController.MainPlayerController_C|GetMainGameWidget _asmain_player_controller)))))

(fn CheckObjectiveKillCount
  (params (Kill%20target :type AI%20Character%20Object%20Reference))
  (for (_array_element _array_index) (Variables|QuestInfo|GetObjectives)
    (LocalVariables|SetArrayIndexLocal _array_index)
    (if (== (Utilities|GetClass (.ObjectiveTarget (Utilities|Struct|BreakObjectiveInfo _array_element))) (Utilities|GetClass Kill%20target))
      (bind _result (Math|Integer|IncrementInt (Variables|QuestInfo|GetCurrentKillCount))
        (:%20%20
          (if (>= _result (.Amount (Utilities|Struct|BreakObjectiveInfo _array_element)))
            (Utilities|Array|SetArrayElem (Variables|QuestInfo|GetObjectives) (LocalVariables|GetArrayIndexLocal) (Utilities|Struct|MakeObjectiveInfo (.description (Utilities|Array|Get(acopy) (Variables|QuestInfo|GetObjectives) (LocalVariables|GetArrayIndexLocal))) (.type (Utilities|Array|Get(acopy) (Variables|QuestInfo|GetObjectives) (LocalVariables|GetArrayIndexLocal))) (.amount (Utilities|Array|Get(acopy) (Variables|QuestInfo|GetObjectives) (LocalVariables|GetArrayIndexLocal))) (.objectivetarget (Utilities|Array|Get(acopy) (Variables|QuestInfo|GetObjectives) (LocalVariables|GetArrayIndexLocal))) true))
            (LocalVariables|SetUpdateQuestStatusLocal true))))))
  (if (LocalVariables|GetUpdateQuestStatusLocal)
    (bind _asmain_player_controller (Utilities|Casting|CastToMainPlayerController (Game|GetPlayerController 0)))
    (Default|UpdateObjectiveState (Variables|/Game/Game/Blueprints/Widgets/MainGameWidget.MainGameWidget_C|GetObjectivesBoxWidget (Variables|/Game/Game/Blueprints/MainPlayerController.MainPlayerController_C|GetMainGameWidget _asmain_player_controller)))))