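; Base world item actor for the inventory system, which the player collects by interacting with it.
; Quest items trigger pickup only when their class matches an objective target in the player's quest log, while other items are picked up directly.
; A successful add to the interactor's Inventory component plays a sound, then notifies each quest of the collection and destroys the actor within that loop.
; UseItem is a stub returning false.
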(event Custom|PickupItem
  ;[0.01042 0.01042 0.01042] Standar pickup
  (bind _sucess (Default|AddItem (Actor|GetComponentbyClass (stale EventInteract Interactor) "/Game/Game/Blueprints/InventorySystem/Inventory.Inventory_C") (Utilities|Struct|MakeItemSlot (Variables|Itemdetails|GetItemDetails) 1)))
  (if _sucess
    (Audio|PlaySound2D (Variables|ItemDetails|GetPickupSound) 1.0 1.0 0.0 0 0)
    (bind _asfirst_person_character (Utilities|Casting|CastToFirstPersonCharacter (Game|GetPlayerCharacter 0)))
    (for _array_element (Variables|/Game/Game/Blueprints/QuestSystem/QuestLog.QuestLog_C|GetQuest (Variables|/Game/Game/Blueprints/FirstPersonCharacter.FirstPersonCharacter_C|GetQuestLog _asfirst_person_character))
      (Default|CallItemCollectionCompleted _array_element self)
      (Actor|DestroyActor))))

(event EventBeginPlay)

(event Collision|EventActorBeginOverlap
  (params (OtherActor :type Actor%20Object%20Reference)))

(event EventTick
  (params (DeltaSeconds :type Float%20%28single-precision%29)))

(event EventInteract
  (params (Interactor :type Actor%20Object%20Reference))
  (if (.questitem (Variables|Itemdetails|GetItemDetails))
    ;[0.01042 0.01042 0.01042] Used for quest item
    (bind _asfirst_person_character (Utilities|Casting|CastToFirstPersonCharacter (Game|GetPlayerCharacter 0)))
    (for _array_element (Variables|/Game/Game/Blueprints/QuestSystem/QuestLog.QuestLog_C|GetQuest (Variables|/Game/Game/Blueprints/FirstPersonCharacter.FirstPersonCharacter_C|GetQuestLog _asfirst_person_character))
      (for _array_element_2 (Variables|/Game/Game/Blueprints/QuestSystem/BaseQuest.BaseQuest_C|GetObjectives _array_element)
        (if (== (Utilities|GetClass (Utilities|Struct|BreakObjectiveInfo _array_element_2)) (Utilities|GetClass self))
          (CallFunction|PickupItem))))
    (else
      ;[0.01042 0.01042 0.01042] Standar pickup
      (CallFunction|PickupItem))))

(fn ConstructionScript)

(fn UseItem
  (return false))