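; MedKit is an inventory item Blueprint that heals the player when used.
; Its UseItem override calls the parent, plays a 2D healing sound, then casts player zero's character to FirstPersonCharacter and adds the item's Health value to that character's Health.
; It returns true after healing, with no clamp to a maximum in this file, and its event graph holds only disabled default events.
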(event EventBeginPlay
  (|CallParentFunction) ; This node is disabled and will not be called.\nDrag off pins to build functionality.
)

(event Collision|EventActorBeginOverlap
  (params (OtherActor :type Actor%20Object%20Reference))
  (|CallParentFunction OtherActor) ; This node is disabled and will not be called.\nDrag off pins to build functionality.
)

(event EventTick
  (params (DeltaSeconds :type Float%20%28single-precision%29))
  (|CallParentFunction DeltaSeconds) ; This node is disabled and will not be called.\nDrag off pins to build functionality.
)

(fn ConstructionScript
  (|CallParentFunction))

(fn UseItem
  (|CallParentFunction)
  (Audio|PlaySound2D (Variables|PickupDetails|GetHealingSound) 1.0 1.0 0.0 0 0)
  (bind _asfirst_person_character (Utilities|Casting|CastToFirstPersonCharacter (Game|GetPlayerCharacter 0)))
  (Variables|/Game/Game/Blueprints/FirstPersonCharacter.FirstPersonCharacter_C|SetHealth _asfirst_person_character (+ (Variables|/Game/Game/Blueprints/FirstPersonCharacter.FirstPersonCharacter_C|GetHealth _asfirst_person_character) (Variables|Pickupdetails|GetHealth)))
  (return true))