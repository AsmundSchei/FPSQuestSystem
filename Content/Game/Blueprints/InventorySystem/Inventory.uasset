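; Player inventory that holds items in a fixed number of slots and toggles its window on the main HUD.
; AddItem tops up a partial stack of stackable items, recursively passing overflow back to itself, or fills the first empty slot with no full-inventory guard.
; Check looks for a single slot holding enough of an item class.
; ToggleInventory creates or removes the window, switching input mode and cursor; the open sound also plays on close.
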(event EventBeginPlay
  (CallFunction|MakeInventory))

(event EventTick
  (params (DeltaSeconds :type Float%20%28single-precision%29)))

(fn ToggleInventory
  (bind _returnvalue (Game|GetPlayerController 0))
  (Audio|PlaySound2D (Variables|InventoryInfo|GetOpenWindowSound) 1.0 1.0 0.0 0 0)
  (Variables|InventoryInfo|GetInventoryWindow
    (:then
      (Widget|RemovefromParent (Variables|InventoryInfo|GetInventoryWindow))
      (Variables|InventoryInfo|SetInventoryWindow 0)
      (Audio|PlaySound2D (Variables|InventoryInfo|GetCloseWindowSound) 1.0 1.0 0.0 0 0)
      (Input|SetInputModeGameOnly _returnvalue)
      (Variables|/Script/Engine.PlayerController|SetbShowMouseCursor _returnvalue false))
    (:else
      (bind _returnvalue_2 (UserInterface|CreateWidget "/Game/Game/Blueprints/InventorySystem/Widgets/InventoryWindowWidget.InventoryWindowWidget_C" 0 self))
      (Variables|InventoryInfo|SetInventoryWindow _returnvalue_2)
      (bind _asmain_player_controller (Utilities|Casting|CastToMainPlayerController _returnvalue))
      (bind _returnvalue_3 (Class|CanvasPanel|AddChildtoCanvas (Variables|/Game/Game/Blueprints/Widgets/MainGameWidget.MainGameWidget_C|GetMainHudCanvasPanel (Variables|/Game/Game/Blueprints/MainPlayerController.MainPlayerController_C|GetMainGameWidget _asmain_player_controller)) (Variables|InventoryInfo|GetInventoryWindow)))
      (Class|CanvasPanelSlot|SetAutoSize _returnvalue_3 true)
      (Class|CanvasPanelSlot|SetAlignment _returnvalue_3 "(X=0.500000,Y=0.500000)")
      (Class|CanvasPanelSlot|SetAnchors _returnvalue_3 (Variables|InventoryInfo|GetWindowAnchor))
      (Class|CanvasPanelSlot|SetPosition _returnvalue_3 (Variables|InventoryInfo|GetWindowPosition))
      (Input|SetInputModeUIOnly _returnvalue (Variables|InventoryInfo|GetInventoryWindow) "LockAlways")
      (Variables|/Script/Engine.PlayerController|SetbShowMouseCursor _returnvalue true))))

(fn MakeInventory
  (Utilities|Array|Resize (Variables|InventoryInfo|GetInventory) (Variables|InventoryInfo|GetNumberOfSlots)))

(fn CreateStack
  (params (AddedItem :type Item%20Slot%20Structure))
  (bind _inventory (Variables|InventoryInfo|GetInventory))
  (Utilities|Array|SetArrayElem _inventory (Utilities|Array|FindItem _inventory (Utilities|Struct|MakeItemSlot "(Name_2_4C29A3D1483D099C7B08F984B63E9095=\"\",Description_4_E23DDB924113A462CA32BDA8E9DC0FBC=\"\",MaxStackSize_7_CD11AAC942221BC641DAB8AD7EEC09E9=0,Durability_10_C7AB4FC94FC637324475F9B4C614B162=0.000000,Consumeable_13_8474E48E427FDCA733358B91B601EDD5=False,StackAble_15_9158D43A44110CBD55D70789DDB74652=False,QuestItem_17_8611F76A46806C5F5ACAB69139865CF6=False,Class_20_838021614B64019FEC6CA6B72BF338A4=None,Image_24_42661ABC459E563ED6C4349705344C4A=None)")) AddedItem))

(fn AddStack
  (params (Item%20 :type Item%20Slot%20Structure) (Slot%20index :type Integer))
  (bind _inventory (Variables|InventoryInfo|GetInventory))
  (bind _inventory_2 (Variables|InventoryInfo|GetInventory))
  (bind _maxstacksize (Utilities|Struct|BreakItem (.item Item%20)))
  (bind _output (Utilities|Array|Get(acopy) _inventory Slot%20index))
  (bind _output_2 (Utilities|Array|Get(acopy) _inventory_2 Slot%20index))
  (bind _output_get (LocalVariables|SetCurrentAmountLocal (.amount _output)))
  (if (> (+ _output_get (Utilities|Struct|BreakItemSlot Item%20)) (.maxstacksize (.item _output)))
    (Utilities|Array|SetArrayElem (Variables|InventoryInfo|GetInventory) Slot%20index (Utilities|Struct|MakeItemSlot (.item Item%20) _maxstacksize))
    (CallFunction|AddItem (Utilities|Struct|MakeItemSlot (.item Item%20) (- (.amount Item%20) (- _maxstacksize (LocalVariables|GetCurrentAmountLocal)))))
    (else
      (Utilities|Array|SetArrayElem _inventory_2 Slot%20index (Utilities|Struct|MakeItemSlot (.item _output_2) (+ (.amount _output_2) (.amount Item%20))))))
  (return true))

(fn AddItem
  (params (ItemAdded :type Item%20Slot%20Structure))
  (if (.stackable (.item ItemAdded))
    (bind _local_stack_index (Utilities|HasPartialStack ItemAdded)
      (:True
        (CallFunction|AddStack ItemAdded _local_stack_index))
      (:False
        (CallFunction|CreateStack ItemAdded :!label _label)))
    (else
      (goto _label)))
  (return true))

(fn Check
  (params (Item :type Base%20Item%20Class%20Reference) (Item%20amount :type Integer))
  (bind _array_element (Utilities|Array|ForEachLoopwithBreak (Variables|InventoryInfo|GetInventory) :!label _label)
    (:LoopBody
      (bind _output_get (LocalVariables|SetAddedToInventoryLocal (and (>= (.amount _array_element) Item%20amount) (== (Utilities|Struct|BreakItem (.item _array_element)) Item))))
      (if _output_get
        (goto _label Break)))
    (:Completed
      (return (LocalVariables|GetAddedToInventoryLocal)))))